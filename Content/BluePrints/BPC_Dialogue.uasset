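; BPC_Dialogue is a dialogue component that shows a named speaker's lines one at a time.
; It creates a WBP_Dialogue widget at BeginPlay, and each Speech call passes it the current line, text delay and name.
; The index then increments, resetting and clearing the widget once it passes the end of the array.
; Speech sets ignore move and look input to false; pause and input-reset nodes are left unconnected.
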(event `self.ReceiveBeginPlay`
  (bind _returnvalue (`|CreateWidget` "/Game/BluePrints/WBP_Dialogue.WBP_Dialogue_C"))
  (set `self.WBP_DialogueRef` _returnvalue))

(event `Speech`
  (bind _returnvalue (`GameplayStatics.GetPlayerController` 0))
  (bind _dialogue (`self.Dialogue`))
  (`Controller.SetIgnoreMoveInput` _returnvalue false)
  (`Controller.SetIgnoreLookInput` _returnvalue false)
  (`/Game/BluePrints/WBP_Dialogue.IncomingText` (`self.WBP_DialogueRef`) (`|GetArrayItem` _dialogue (`self.CurrentDialogue`)) (`self.TextDelay`) (`self.Name`))
  (bind _result (`/Engine/EditorBlueprintResources/StandardMacros.IncrementInt` (`self.CurrentDialogue`))
    (:`  `
      (if (>= _result (+ (`KismetArrayLibrary.Array_Length` _dialogue) 1))
        (set `self.CurrentDialogue` 0)
        (`/Game/BluePrints/WBP_Dialogue.ClearScreen` (`self.WBP_DialogueRef`))))))