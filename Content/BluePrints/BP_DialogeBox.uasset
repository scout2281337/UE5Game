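; BP_DialogeBox is an interactable Blueprint that plays dialogue through its BPCDialogue component.
; Each Interact event calls Speech and increments the WasShown counter, until that counter exceeds the length of the component's Dialogue, allowing one call more than that length.
; A second Speech call is left unconnected, and the construction script is empty.
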(event `/Game/BluePrints/Interfaces/I_Interactable.Interact`
  (params (Player :type "/Game/BluePrints/BP_FirstPersonCharacter Object Reference"))
  (if (not (> (`self.WasShown`) (`KismetArrayLibrary.Array_Length` (`/Game/BluePrints/BPC_Dialogue.Dialogue` (`self.BPC_Dialogue`)))))
    (`/Game/BluePrints/BPC_Dialogue.Speech` (`self.BPC_Dialogue`))
    (bind _result (`/Engine/EditorBlueprintResources/StandardMacros.IncrementInt` (`self.WasShown`))
      (:`  `
        (set `self.WasShown` _result)))))

(fn `UserConstructionScript`)