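; BP_Door is an interactable door that swings open and closed and can require a matching key.
; Interact plays a sound and flip-flops a Timeline forward or in reverse to drive the root's yaw.
; DoorID 0 needs no key; otherwise a matching ID in the player's Keys sets IsOpen, which acts as an unlocked flag.
; Unlocking does not move the door, so it swings on a later interaction.
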(event `/Game/BluePrints/Interfaces/I_Interactable.Interact`
  (params (Player :type "/Game/BluePrints/BP_FirstPersonCharacter Object Reference"))
  (if (`self.IsOpen`)
    (`self.PlaySound` :!label _label)
    (`/Engine/EditorBlueprintResources/StandardMacros.FlipFlop`
      (:`A`
        (bind (_direction _curve) (`Timeline|Timeline` :!label _label_2)
          (:`Update`
            (`SceneComponent.K2_SetRelativeRotation` (`self.DefaultSceneRoot`) (`KismetMathLibrary.MakeRotator` 0.0 0.0 _curve) false false))))
      (:`B`
        (goto _label_2 :!via `Reverse`)))
    (elif (== (`self.DoorID`) 0)
      (goto _label)
      (else
        (for _array_element (`/Game/BluePrints/BP_FirstPersonCharacter.Keys` Player)
          (if (== _array_element (`self.DoorID`))
            (set `self.IsOpen` true)
            (break)))))))

(fn `PlaySound`
  (`GameplayStatics.PlaySoundAtLocation` "/Game/Fab/Sound/Door_Cue.Door_Cue" (`SceneComponent.K2_GetComponentLocation` (`self.DefaultSceneRoot`)) (struct) 1.0 1.0 0.0 null null null null))

(fn `UserConstructionScript`)