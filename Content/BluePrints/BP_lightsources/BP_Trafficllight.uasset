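; BP_Trafficllight is a traffic light Blueprint that blinks its three point lights at random.
; On BeginPlay it gathers the lights into an array and runs an endless loop: light a random one, wait a random delay, then switch off a random one.
; The two picks are independent, so several lights can be lit at once rather than following a red-amber-green sequence.
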(event `self.ReceiveBeginPlay`
  (bind _outitem (`KismetArrayLibrary.Array_Random` (`self.array`)))
  (set `self.array` (`|MakeArray` (`self.PointLight2`) (`self.PointLight1`) (`self.PointLight`)))
  (`LightComponent.SetIntensity` _outitem 2000.0 :!label _label)
  (`KismetSystemLibrary.Delay` (`KismetMathLibrary.RandomFloatInRange` 0.2 4.0))
  (`LightComponent.SetIntensity` _outitem 0.0)
  (goto _label))

(fn `UserConstructionScript`)