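; BP_Monster is an enemy character that triggers a jumpscare when the player enters its sphere.
; On overlap with BP_FirstPersonCharacter, it disables that player's input, turns their view toward the monster, plays a zombie headbutt animation and a 2D scream sound.
; Helper functions return a random entry from its Spots array and map a movement state, from idle to sprint, to max walk speed.
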(event `self.Sphere.OnComponentBeginOverlap`
  (params (OverlappedComponent :type "PrimitiveComponent Object Reference") (OtherActor :type "Actor Object Reference") (OtherComp :type "PrimitiveComponent Object Reference") (OtherBodyIndex :type Integer) (bFromSweep :type Boolean) (SweepResult :type "HitResult Structure (by ref)"))
  (bind _returnvalue (`GameplayStatics.GetPlayerController` 0))
  (bind _asbp_first_person_character (cast `/Game/BluePrints/BP_FirstPersonCharacter` OtherActor))
  (`self.DisableInput` _asbp_first_person_character _returnvalue)
  (`Controller.SetControlRotation` _returnvalue (`KismetMathLibrary.FindLookAtRotation` (`self.K2_GetActorLocation` _asbp_first_person_character) (`self.K2_GetActorLocation`)))
  (`SkeletalMeshComponent.PlayAnimation` (`self.Mesh`) "/Game/Monster/Model/Zombie_Headbutt.Zombie_Headbutt" false)
  (`GameplayStatics.PlaySound2D` "/Game/Fab/Sound/AAAAAAAAAAAAAA_Cue.AAAAAAAAAAAAAA_Cue" 1.0 1.0 0.0 null null))

(fn `GetRandomSpot`
  (returns (Spot :type "Actor Object Reference"))
  (bind _spots (`self.Spots`))
  (return (`|GetArrayItem` _spots (`KismetMathLibrary.RandomInteger` (`KismetArrayLibrary.Array_Length` _spots)))))

(fn `SetMovement`
  (params (Movement :type "/Game/Monster/E_MonsterMovement Enum" :default "NewEnumerator0"))
  (returns (Speed :type "Float (double-precision)"))
  (bind _output_get (set `CharacterMovementComponent.MaxWalkSpeed` (select `/Game/Monster/E_MonsterMovement` Movement :`NewEnumerator1` 200.0 :`NewEnumerator2` 350.0 :`NewEnumerator3` 500.0 :!type "Float (single-precision)") (`self.CharacterMovement`)))
  (return _output_get))

(fn `UserConstructionScript`)